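; BP_MRControls is a keyboard-driven actor for switching between VR and mixed reality views using OculusXR passthrough.
; N alternates the environment blend mode between Opaque and AlphaBlend, then creates or destroys persistent passthrough based on the MRBackground flag.
; B flips that flag and shows or hides VROnlyObjects, leaving passthrough itself unchanged until N is pressed.
; EndPlay destroys passthrough, and a FreeCameraPawn lookup sits unconnected.
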(event `self.ReceiveBeginPlay`
  (`self.EnableInput` (`GameplayStatics.GetPlayerController` 0)))

(event `Key|N`
  (params (Key :type "Key Structure"))
  ;[1 1 1] MRToggle
  (:`Pressed`
    (`/Engine/EditorBlueprintResources/StandardMacros.FlipFlop`
      (:`A`
        (`OpenXRBlueprintFunctionLibrary.SetEnvironmentBlendMode` "Opaque"))
      (:`B`
        (`OpenXRBlueprintFunctionLibrary.SetEnvironmentBlendMode` "AlphaBlend")))
    (if (`self.MRBackground`)
      (`OculusXRPassthroughSubsystem.InitializePersistentPassthrough` :`self` (subsystem `OculusXRPassthroughSubsystem`))
      (else
        (`OculusXRPassthroughSubsystem.DestroyPersistentPassthrough` (subsystem `OculusXRPassthroughSubsystem`) :!label _label)))))

(event `self.ReceiveEndPlay`
  (params (EndPlayReason :type "EEndPlayReason Enum" :default "Destroyed"))
  (goto _label))

(event `Key|B`
  (params (Key :type "Key Structure"))
  ;[1 1 1] BackgroundToggle
  (:`Pressed`
    (bind _output_get (set `self.MRBackground` (not (`self.MRBackground`))))
    (for _array_element (`self.VROnlyObjects`)
      (`SceneComponent.SetVisibility` (`Actor.RootComponent` _array_element) (not _output_get) true))))

(fn `UserConstructionScript`)